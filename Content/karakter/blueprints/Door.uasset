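; Door Blueprint that swings open and shut, with sounds for opening, closing and knocking.
; The Openclose event alternates through a FlipFlop, capturing the root rotation and a target 90 degrees further in yaw on opening.
; The Kapiac timeline lerps the root between them, playing slowly to open and reversing faster to close, with positional sounds.
; A separate Kapical event plays a 2D knock sound.
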(event Custom|Openclose
  (bind _defaultsceneroot (Variables|Default|GetDefaultSceneRoot))
  (bind _returnvalue (Transformation|GetWorldRotation _defaultsceneroot))
  (bind (_roll _pitch _yaw) (Math|Rotator|BreakRotator _returnvalue))
  (Utilities|FlowControl|FlipFlop
    (:A
      (Variables|Default|Setbaserotation _returnvalue)
      (Variables|Default|SetTargetrotation (Math|Rotator|MakeRotator _roll _pitch (+ _yaw 9e+01)))
      (Components|Timeline|SetPlayRate (Variables|Default|GetKapiac) 0.35)
      (Audio|PlaySoundatLocation "/Game/karakter/sesler/doorOpen.doorOpen" (Transformation|GetWorldLocation (Variables|Default|GetDoor)) "0, 0, 0" 1.0 1.0 0.0 0 0 0)
      (bind _kapiacma (Timeline|Kapiac Play)
        (:Update
          (Transformation|SetWorldRotation (Variables|Default|GetDefaultSceneRoot) (Math|Rotator|Lerp(Rotator) (Variables|Default|Getbaserotation) (Variables|Default|GetTargetrotation) _kapiacma) false false))))
    (:B
      (Components|Timeline|SetPlayRate (Variables|Default|GetKapiac) 1.0)
      (Audio|PlaySoundatLocation "/Game/karakter/sesler/doorClose.doorClose" (Transformation|GetWorldLocation (Variables|Default|GetDoor)) "0, 0, 0" 1.0 1.0 0.0 0 0 0)
      (Timeline|Kapiac Reverse))))

(event Custom|Kapical
  (Audio|PlaySound2D "/Game/karakter/sesler/Knock_Knock.Knock_Knock" 1.0 1.0 0.0 0 0))

(fn ConstructionScript)